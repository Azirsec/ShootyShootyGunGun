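; BP_Gate is an upgrade gate that sells the player a stat boost on overlap for a point cost.
; It casts to BP_ThirdPersonCharacter, spends GateCost, then switches on GateUpgrade to raise damage, health, regen, fire rate, speed or burn damage.
; A successful purchase destroys the gate's parent actor.
; SetTextDisplay shows the upgrade name on a TextRender, while the random-upgrade logic in the event graph is disconnected.
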(event EventBeginPlay)

(event EventTick
  (params (DeltaSeconds :type Float%20%28single-precision%29)))

(event Collision|EventActorBeginOverlap
  (params (OtherActor :type Actor%20Object%20Reference))
  (bind _asbp_third_person_character (Utilities|Casting|CastToBP_ThirdPersonCharacter OtherActor))
  (bind _buy_succeed (Default|SpendPoints _asbp_third_person_character (Variables|Default|GetGateCost)))
  (Default|UpdatePoints _asbp_third_person_character)
  (Development|PrintString (Utilities|String|ToString(Boolean) _buy_succeed))
  (if _buy_succeed
    (switch Utilities|FlowControl|Switch|SwitchonUpgradeOptions (Variables|Default|GetGateUpgrade)
      (:NewEnumerator0
        (Default|IncreaseDamage _asbp_third_person_character 1e+01))
      (:NewEnumerator1
        (Default|IncreaseMaxHealth _asbp_third_person_character 1e+01))
      (:NewEnumerator2
        (Default|IncreaseHealthRegen _asbp_third_person_character 2.0))
      (:NewEnumerator3
        (Default|IncreaseFireRate _asbp_third_person_character 0.5))
      (:NewEnumerator4
        (Default|IncreaseMoveSpeed _asbp_third_person_character 2e+02))
      (:NewEnumerator5
        (Default|IncreaseBurnDamage _asbp_third_person_character 5.0)))
    (Actor|DestroyActor (Actor|GetParentActor))))

(fn ConstructionScript)

(fn SetTextDisplay
  (Rendering|Components|TextRender|SetText (Variables|Default|GetTextRender) (Utilities|Text|ToText(String) (Utilities|String|EnumtoString (Variables|Default|GetGateUpgrade)))))