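; BP_DualGate is an environment actor that pairs two BP_Gate child actors, each offering a different random upgrade.
; On BeginPlay it randomly picks an Offensive or Defensive category, then draws one of that category's three upgrades for each side.
; The right gate rerolls until it differs from the left.
; Both upgrades are then pushed into the LeftGate and RightGate child actors, which refresh their text displays.
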(event EventBeginPlay
  (bind _returnvalue (Math|Random|RandomInteger 3))
  (bind _returnvalue_2 (Math|Random|RandomInteger 3))
  (bind _returnvalue_3 (Utilities|Select :Index _returnvalue :Option%200 "NewEnumerator1" :Option%201 "NewEnumerator2" :Option%202 "NewEnumerator4"))
  (bind _returnvalue_4 (Utilities|Select :Index _returnvalue_2 :Option%200 "NewEnumerator0" :Option%201 "NewEnumerator3" :Option%202 "NewEnumerator5"))
  (bind _output_get (Variables|Default|SetUpgradeType (Utilities|Select :Index (Math|Random|RandomInteger 2) :Option%200 "NewEnumerator0" :Option%201 "NewEnumerator1")))
  (switch Utilities|FlowControl|Switch|SwitchonUpgradeTypes _output_get
    (:NewEnumerator0
      (bind _output_get_2 (Variables|Default|SetLGUpgrade _returnvalue_4))
      (bind _output_get_3 (Variables|Default|SetRGUpgrade _returnvalue_4 :!label _label))
      (if (Utilities|Enum|Equal(Enum) _output_get_2 _output_get_3)
        (goto _label)
        (else
          _)))
    (:NewEnumerator1
      (bind _output_get_4 (Variables|Default|SetLGUpgrade _returnvalue_3))
      (bind _output_get_5 (Variables|Default|SetRGUpgrade _returnvalue_3 :!label _label_2))
      (if (Utilities|Enum|Equal(Enum) _output_get_4 _output_get_5)
        (goto _label_2)
        (else
          _))))
  (bind _asbp_gate (Utilities|Casting|CastToBP_Gate (Variables|/Script/Engine.ChildActorComponent|GetChildActor (Variables|Default|GetLeftGate))))
  (Variables|/Game/Interactive_Objects/Environment/BP_Gate.BP_Gate_C|SetGateUpgrade _asbp_gate (Variables|Default|GetLGUpgrade))
  (Default|SetTextDisplay _asbp_gate)
  (bind _asbp_gate_2 (Utilities|Casting|CastToBP_Gate (Variables|/Script/Engine.ChildActorComponent|GetChildActor (Variables|Default|GetRightGate))))
  (Variables|/Game/Interactive_Objects/Environment/BP_Gate.BP_Gate_C|SetGateUpgrade _asbp_gate_2 (Variables|Default|GetRGUpgrade))
  (Default|SetTextDisplay _asbp_gate_2))

(fn ConstructionScript)